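; Master elevator lift that moves a wall-panel platform vertically by TravelDistance when a pawn is on its pressure plate.
; Plate overlaps request movement through ServerStartElevator, while a looping authority-only timer with slightly randomized interval also checks for waiting passengers.
; ToggleElevator plays or reverses a timeline based on extent and GoesUp, with pitch-varied audio.
; On finishing, it updates travel state and optionally auto-returns from the extent after a delay.
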(event OnComponentBeginOverlap(PressurePlate)
  (params (OverlappedComponent :type Primitive%20Component%20Object%20Reference) (OtherActor :type Actor%20Object%20Reference) (OtherComp :type Primitive%20Component%20Object%20Reference) (OtherBodyIndex :type Integer) (bFromSweep :type Boolean) (SweepResult :type Hit%20Result%20Structure%20%28by%20ref%29))
  ;[1 1 1] Elevator Functionality
  (if (not (Variables|Default|GetIsTravelling))
    (Utilities|Casting|CastToPawn OtherActor)
    (CallFunction|RequestElevatorMovement)))

(event Custom|Return
  (bind _audio (Variables|Default|GetAudio))
  ;[1 1 1] Elevator Functionality
  (if true
    (Audio|Components|Audio|SetPitchMultiplier _audio (Math|Random|RandomFloatinRange 0.95 1.0))
    (Audio|Components|Audio|Play _audio 0.0)
    (bind (_direction _movement) (Timeline|ElevatorAnimation Reverse)
      (:Update
        (Transformation|SetRelativeLocation (Variables|Default|GetSM_Wall_Panel_Flat) (Math|Vector|MakeVector 0.0 0.0 (* _movement (Variables|Default|GetTravelDistance))) false false))
      (:Finished
        (Variables|Default|SetIsTravelling false)
        (Variables|Default|SetIsAtExtent (Utilities|Enum|Equal(Enum) _direction "Forward"))
        (if (Variables|Default|GetAutoReturn)
          (Utilities|FlowControl|Delay 3.0)
          (if (and (not (Variables|Default|GetIsTravelling)) (Variables|Default|GetIsAtExtent))
            (CallFunction|Return)))))
    (else
      (Audio|Components|Audio|SetPitchMultiplier _audio (Math|Random|RandomFloatinRange 1.0 1.05))
      (Audio|Components|Audio|Play _audio 0.0)
      (Timeline|ElevatorAnimation Play))))

(event Custom|Retrieve
  (bind _audio (Variables|Default|GetAudio))
  ;[1 1 1] Elevator Functionality
  (if (Variables|Default|GetGoesUp)
    (Audio|Components|Audio|SetPitchMultiplier _audio (Math|Random|RandomFloatinRange 1.0 1.05))
    (Audio|Components|Audio|Play _audio 0.0)
    (bind (_direction _movement) (Timeline|ElevatorAnimation Play)
      (:Update
        (Transformation|SetRelativeLocation (Variables|Default|GetSM_Wall_Panel_Flat) (Math|Vector|MakeVector 0.0 0.0 (* _movement (Variables|Default|GetTravelDistance))) false false))
      (:Finished
        (Variables|Default|SetIsTravelling false)
        (Variables|Default|SetIsAtExtent (Utilities|Enum|Equal(Enum) _direction "Forward"))
        (if (Variables|Default|GetAutoReturn)
          (Utilities|FlowControl|Delay 3.0)
          (if (and (not (Variables|Default|GetIsTravelling)) (Variables|Default|GetIsAtExtent))
            (CallFunction|Return)))))
    (else
      (Audio|Components|Audio|SetPitchMultiplier _audio (Math|Random|RandomFloatinRange 0.95 1.0))
      (Audio|Components|Audio|Play _audio 0.0)
      (Timeline|ElevatorAnimation Reverse))))

(event Custom|RequestElevatorMovement
  ;[1 1 1] Elevator Functionality
  (CallFunction|ServerStartElevator))

(event Custom|ToggleElevator
  (bind _audio (Variables|Default|GetAudio))
  ;[1 1 1] Elevator Functionality
  (Variables|Default|SetIsTravelling true)
  (if (Variables|Default|GetIsAtExtent)
    (if true
      (Audio|Components|Audio|SetPitchMultiplier _audio (Math|Random|RandomFloatinRange 0.95 1.0) :!label _label)
      (Audio|Components|Audio|Play _audio 0.0)
      (bind (_direction _movement) (Timeline|ElevatorAnimation Reverse)
        (:Update
          (Transformation|SetRelativeLocation (Variables|Default|GetSM_Wall_Panel_Flat) (Math|Vector|MakeVector 0.0 0.0 (* _movement (Variables|Default|GetTravelDistance))) false false))
        (:Finished
          (Variables|Default|SetIsTravelling false)
          (Variables|Default|SetIsAtExtent (Utilities|Enum|Equal(Enum) _direction "Forward"))
          (if (Variables|Default|GetAutoReturn)
            (Utilities|FlowControl|Delay 3.0)
            (if (and (not (Variables|Default|GetIsTravelling)) (Variables|Default|GetIsAtExtent))
              (CallFunction|Return)))))
      (else
        (Audio|Components|Audio|SetPitchMultiplier _audio (Math|Random|RandomFloatinRange 1.0 1.05) :!label _label_2)
        (Audio|Components|Audio|Play _audio 0.0)
        (Timeline|ElevatorAnimation Play)))
    (elif (Variables|Default|GetGoesUp)
      (goto _label_2)
      (else
        (goto _label)))))

(event Custom|ServerStartElevator
  ;[1 1 1] Elevator Functionality
  (CallFunction|ToggleElevator))

(event Custom|CheckForPassengers
  ;[1 1 1] Check for passengers
  (if (not (Variables|Default|GetIsTravelling))
    (if (Utilities|Array|IsValidIndex (Collision|GetOverlappingActors (Variables|Default|GetPressurePlate) "/Script/Engine.Pawn" :!class /Script/Engine.PrimitiveComponent))
      (CallFunction|ToggleElevator))))

(event EventBeginPlay
  ;[0 1 0.003062] Begin Play
  (Networking|SwitchHasAuthority
    (:Authority
      (Utilities|Time|SetTimerbyEvent (delegate Custom|CheckForPassengers) (Math|Random|RandomFloatinRange 2.9 3.1) true))))

(fn ConstructionScript)