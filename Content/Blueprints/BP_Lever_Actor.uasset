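; BP_Lever_Actor is a VR lever that acts as a switch in an electrical interface system.
; It stores the CurrentFlow value received through its CurrentStateChange event.
; When the VRLever component changes state, it messages every entry in ElectricalTargets with itself as provider, the lever status and the stored flow.
; GetAngle reports the lever's roll, both raw and relative to its initial rotation.
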(event OnLeverStateChanged(VRLever)
  (params (LeverStatus :type Boolean) (LeverStatusType :type EVRInteractibleLeverEventType%20Enum :default "LeverPositive") (LeverAngleAtTime :type Float%20%28single-precision%29) (FullLeverAngleAtTime :type Float%20%28single-precision%29))
  ;[1 1 1] Electrical Interface Events
  (for _array_element (Variables|Default|GetElectricalTargets)
    (Class|ElectricalObject|CurrentStateChange(Message) _array_element self LeverStatus (Variables|Default|GetCurrentFlow))))

(event EventCurrentStateChange
  (params (CurrentProvider :type Object%20Object%20Reference) (ElectricalState :type Boolean) (CurrentFlow :type Float%20%28single-precision%29))
  ;[1 1 1] Electrical Interface Events
  (Variables|Default|SetCurrentFlow CurrentFlow))

(fn ConstructionScript)

(fn GetAngle
  (bind _vrlever (Variables|Default|GetVRLever))
  (bind _relativerotation (Variables|/Script/Engine.SceneComponent|GetRelativeRotation _vrlever))
  (return (- (.roll _relativerotation) (Variables|Default|GetInitialRot)) (.roll _relativerotation)))