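; Physics mop prop that paints a black brush onto render targets of surfaces it hits, with a return to its starting transform.
; Server hits multicast the mop socket location with velocity-scaled brush size and random rotation.
; Remote clients trace down, find the collision UV and pass a dynamic brush material to the hit actor to draw.
; Android flips the V coordinate.
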(event Custom|Server_Mop
  ;[1 1 1] Server Events
  (CallFunction|MultiMop (Transformation|GetSocketLocation (Variables|Default|GetSkeletalMeshComponent) "MopEndSocket") (Math|Vector|MakeVector (Math|Float|MapRangeClamped (Math|Vector|VectorLength (Transformation|GetVelocity)) 0.0 1.2e+03 0.05 0.15) (Math|Random|RandomFloatinRange 0.0 1.0) 0.0)))

(event Custom|Multi_Mop
  (params (Location :type Vector) (Attributes :type Vector))
  (bind _mi_drawbrush (Variables|Default|GetMI_DrawBrush))
  ;[1 1 1] Multicast Events
  (Networking|SwitchHasAuthority ; Only on clients
    (:Remote
      (bind _outhit (Collision|LineTraceByChannel (Transformation|GetSocketLocation (Variables|Default|GetSkeletalMeshComponent) "MopEndSocket") (+ Location "0, 0,-40.000000") "TraceTypeQuery1" true 0 "ForOneFrame" true "(R=1.000000,G=0.000000,B=0.000000,A=1.000000)" "(R=0.000000,G=1.000000,B=0.000000,A=1.000000)" 3.0))
      (if (.ReturnValue (Class|GameplayStatics|FindCollisionUV _outhit))
        (Rendering|Material|SetVectorParameterValue _mi_drawbrush "UVLocation" (Utilities|Struct|MakeLinearColor (.x (.UV (Class|GameplayStatics|FindCollisionUV _outhit))) (Math|Float|Absolute(Float) (- (Variables|Default|GetFlipUVScalar) (.y (.UV (Class|GameplayStatics|FindCollisionUV _outhit))))) (.y Attributes) 1.0) :!class /Script/Engine.MaterialInstanceDynamic)
        (Rendering|Material|SetScalarParameterValue _mi_drawbrush "BrushSize" (.x Attributes) :!class /Script/Engine.MaterialInstanceDynamic)
        (Rendering|Material|SetVectorParameterValue :self _mi_drawbrush :ParameterName "Color" :!class /Script/Engine.MaterialInstanceDynamic)
        (Class|RenderTargetInterface|DrawBrushtoRenderTarget(Message) (.HitActor (Collision|BreakHitResult _outhit)) _mi_drawbrush)))))

(event Custom|ServerReturn
  (bind _skeletalmeshcomponent (Variables|Default|GetSkeletalMeshComponent))
  ;[1 1 1] Server Events
  (Class|PrimitiveComponent|SetAllPhysicsAngularVelocityinDegrees _skeletalmeshcomponent (Math|Vector|MakeVector 0.0 0.0 0.0) false)
  (Physics|SetPhysicsLinearVelocity _skeletalmeshcomponent "0, 0, 0" false "None")
  (Transformation|SetWorldTransform _skeletalmeshcomponent (Variables|Default|GetInitialWorldTransform) false false))

(event EventSetReturnLocation
  ;[1 1 1] Interface Events
  (Variables|Default|SetInitialWorldTransform (Transformation|GetWorldTransform (Variables|Default|GetSkeletalMeshComponent))))

(event Collision|EventHit
  (params (MyComp :type Primitive%20Component%20Object%20Reference) (Other :type Actor%20Object%20Reference) (OtherComp :type Primitive%20Component%20Object%20Reference) (bSelfMoved :type Boolean) (HitLocation :type Vector :default "0, 0, 0") (HitNormal :type Vector :default "0, 0, 0") (NormalImpulse :type Vector :default "0, 0, 0") (Hit :type Hit%20Result%20Structure%20%28by%20ref%29))
  ;[1 1 1] Collision Event Hits
  (Networking|SwitchHasAuthority
    (:Authority
      (CallFunction|ServerMop))))

(event EventReturn
  ;[1 1 1] Interface Events
  (CallFunction|ServerReturn))

(event EventBeginPlay
  ;[0.01644 0.2 0] Begin Play
  (Utilities|FlowControl|Sequence
    (:then_0
      (Networking|SwitchHasAuthority
        (:Authority
          (CallFunction|SetReturnLocation))))
    (:then_1
      (switch string (Game|GetPlatformName)
        (:Android
          (Variables|Default|SetFlipUVScalar 1.0))))))

(fn ConstructionScript
  (bind _returnvalue (Rendering|Material|CreateDynamicMaterialInstance (Variables|Default|GetDrawBrush) "None" :!class /Script/Engine.KismetMaterialLibrary))
  (Variables|Default|SetMI_DrawBrush _returnvalue))

(fn GetReturnLocation
  (return ""))