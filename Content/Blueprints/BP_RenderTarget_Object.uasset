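; Paintable static mesh actor that lets brush materials draw onto its own render target at runtime.
; On BeginPlay it creates a render target and feeds it into a dynamic instance of the mesh's material.
; Interface events draw a brush material directly, or line trace between two points, convert the hit to a collision UV and set the brush's UVLocation before drawing.
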(event EventBeginPlay
  (bind _staticmesh (Variables|Default|GetStaticMesh))
  ;[0 1 0] Begin Play
  (bind _returnvalue (Rendering|CreateRenderTarget2D (Variables|RenderTarget|GetRT_Width) (Variables|RenderTarget|GetRT_Height) "RTF_RGBA8" "(R=0.000000,G=0.000000,B=0.000000,A=0.000000)"))
  (bind _output_get (Variables|RenderTarget|SetT_RenderTarget _returnvalue))
  (bind _returnvalue_2 (Rendering|Material|CreateDynamicMaterialInstance (Rendering|Material|GetMaterial _staticmesh 0) "None" "None" :!class /Script/Engine.KismetMaterialLibrary))
  (bind _output_get_2 (Variables|RenderTarget|SetMI_PaintableMaterial _returnvalue_2))
  (Rendering|Material|SetMaterial _staticmesh 0 _output_get_2)
  (Rendering|Material|SetTextureParameterValue _output_get_2 "RenderTarget" _output_get))

(event EventDrawBrushtoRenderTarget
  (params (BrushMaterial :type Material%20Instance%20Dynamic%20Object%20Reference%20%28by%20ref%29))
  ;[1 1 1] Interface Events
  (Rendering|DrawMaterialtoRenderTarget (Variables|RenderTarget|GetT_RenderTarget) BrushMaterial))

(event EventTrytoDrawBrushtoRenderTarget
  (params (BrushMaterial :type Material%20Instance%20Dynamic%20Object%20Reference%20%28by%20ref%29) (StartLocation :type Vector :default "0, 0, 0") (EndLocation :type Vector :default "0, 0, 0"))
  ;[1 1 1] Interface Events
  (bind _outhit (Collision|LineTraceByChannel StartLocation EndLocation "TraceTypeQuery1" true 0 "None" false "(R=1.000000,G=0.000000,B=0.000000,A=1.000000)" "(R=0.000000,G=1.000000,B=0.000000,A=1.000000)" 1.0))
  (if (.ReturnValue (Class|GameplayStatics|FindCollisionUV _outhit))
    (Rendering|Material|SetVectorParameterValue BrushMaterial "UVLocation" (Utilities|Struct|MakeLinearColor (.x (.UV (Class|GameplayStatics|FindCollisionUV _outhit))) (.y (.UV (Class|GameplayStatics|FindCollisionUV _outhit))) 0.0 1.0) :!class /Script/Engine.MaterialInstanceDynamic)
    (Rendering|DrawMaterialtoRenderTarget (Variables|RenderTarget|GetT_RenderTarget) BrushMaterial)))

(fn ConstructionScript)