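; Aim-trainer target grid that spawns randomly sized BP_TargetCube actors on a centred vertical grid and tracks shooting accuracy.
; Respawn calls itself until MaxTargets exist, relying on collision-checked spawning to reject occupied spots.
; Each target death triggers a respawn, adds score and selects the size range for its score tier.
; Projectiles overlapping MissBox count as misses, updating score and accuracy text; target-count cycling logic is unconnected.
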(event OnComponentBeginOverlap(MissBox)
  (params (OverlappedComponent :type Primitive%20Component%20Object%20Reference) (OtherActor :type Actor%20Object%20Reference) (OtherComp :type Primitive%20Component%20Object%20Reference) (OtherBodyIndex :type Integer) (bFromSweep :type Boolean) (SweepResult :type Hit%20Result%20Structure%20%28by%20ref%29))
  ;[1 1 1] MissBox Overlap
  (Utilities|Casting|CastToFirstPersonProjectile OtherActor)
  (Math|Integer|IncrementInt (Variables|Default|GetMissScore)
    (:%20%20
      (CallFunction|CalculateAccuracy))))

(event Custom|Respawn
  (bind _scene (Variables|Default|GetScene))
  (bind _gridrows (Variables|Default|GetGridRows))
  (bind _gridcollums (Variables|Default|GetGridCollums))
  (bind _targetsizemin (Variables|Default|GetTargetSizeMin))
  (bind _targetsizemax (Variables|Default|GetTargetSizeMax))
  (bind _returnvalue (Math|Random|RandomFloatinRange _targetsizemin _targetsizemax))
  (bind _returnvalue_2 (Transformation|GetWorldLocation _scene))
  (bind _returnvalue_3 (* _gridrows _gridcollums))
  (bind _returnvalue_4 (- _returnvalue_3 1))
  (bind _returnvalue_5 (Math|Random|RandomIntegerinRange 0 _returnvalue_4))
  ;[1 1 1] Spawn and Respawn Targets
  (Development|PrintString (Utilities|String|ToString(Integer) _returnvalue_5) true true "(R=0.000000,G=1.000000,B=0.037633,A=1.000000)")
  (bind _returnvalue_6 (Game|SpawnActorfromClass "/Game/Blueprints/BP_TargetCube.BP_TargetCube_C" (Math|Transform|MakeTransform (Math|Vector|MakeVector (+ (* (Math|Integer|%(Integer) _returnvalue_5 (Variables|Default|GetGridRows)) (Variables|Default|GetGridSpacing)) (.x _returnvalue_2)) (.y _returnvalue_2) (+ (* (/ _returnvalue_5 (Variables|Default|GetGridRows)) (Variables|Default|GetGridSpacing)) (.z _returnvalue_2))) "0, 0, 0" (Math|Vector|MakeVector _returnvalue _returnvalue _returnvalue)) "DontSpawnIfColliding" 0 _returnvalue_5 0))
  (Utilities|IsValid _returnvalue_6
    (:Is%20Valid
      (Math|Integer|IncrementInt (Variables|Default|GetNumberOfTargets)
        (:%20%20
          (EventDispatchers|BindEventtoTargetDied _returnvalue_6 (delegate Custom|TargetDiedEvent)))))
    (:Is%20Not%20Valid
      _))
  (if (< (Variables|Default|GetNumberOfTargets) (Variables|Default|GetMaxTargets))
    (CallFunction|Respawn)))

(event Custom|TargetDiedEvent
  (params (Index :type Integer))
  (bind _score (Variables|Default|GetScore))
  ;[1 1 1] Spawn and Respawn Targets
  (Math|Integer|DecrementInt (Variables|Default|GetNumberOfTargets)
    (:%20%20
      (CallFunction|Respawn)
      (CallFunction|IncreaseScore)
      (CallFunction|CalculateAccuracy)
      ;[1 1 1] Set Target Box Min Scale
      (if (< _score (Variables|Default|GetFirstScaleDownScore))
        (Variables|Default|SetTargetSizeMin (Variables|Default|GetFirstScaleMin))
        (Variables|Default|SetTargetSizeMax (Variables|Default|GetFirstScaleMax))
        (elif (< _score (Variables|Default|GetSecondScaleDownScore))
          (Variables|Default|SetTargetSizeMin (Variables|Default|GetSecondScaleMin))
          (Variables|Default|SetTargetSizeMax (Variables|Default|GetSecondScaleMax))
          (elif (< _score (Variables|Default|GetThirdScaleDownScore))
            (Variables|Default|SetTargetSizeMin (Variables|Default|GetThirdScaleMin))
            (Variables|Default|SetTargetSizeMax (Variables|Default|GetThirdScaleMax))
            (elif (< _score (Variables|Default|GetFourthScaleDownScore))
              (Variables|Default|SetTargetSizeMin (Variables|Default|GetFourthScaleMin))
              (Variables|Default|SetTargetSizeMax (Variables|Default|GetFourthScaleMax))
              (elif (< _score (Variables|Default|GetFifthScaleDownScore))
                (Variables|Default|SetTargetSizeMin (Variables|Default|GetFifthScaleMin))
                (Variables|Default|SetTargetSizeMax (Variables|Default|GetFifthScaleMax))
                (else
                  (Variables|Default|SetSixthScaleMin (Variables|Default|GetSixthScaleMin))
                  (Variables|Default|SetTargetSizeMax (Variables|Default|GetSixthScaleMax)))))))))))

(event Custom|Increase%20Score
  ;[1 1 1] Increase Score
  (Math|Integer|IncrementInt (Variables|Default|GetScore)
    (:%20%20
      (CallFunction|CalculateAccuracy))))

(event Custom|CalculateAccuracy
  (bind _score (Variables|Default|GetScore))
  (bind _missscore (Variables|Default|GetMissScore))
  (bind _returnvalue (+ _score _missscore))
  ;[1 1 1] Calculate Accuracy
  (Rendering|Components|TextRender|SetText (Variables|Default|GetScoreText) (Utilities|Text|FormatText "{A}/{B}" (Variables|Default|GetScore) (Variables|Default|GetMissScore)))
  (if (> _returnvalue 0)
    (Rendering|Components|TextRender|SetText (Variables|Default|GetAccuracyPercentText) (Utilities|Text|FormatText "Accuracy: {score}%" (Math|Float|Truncate (* (/ (Math|Conversions|ToFloat(Integer) _score) (Math|Conversions|ToFloat(Integer) _returnvalue)) 1e+02))))))

(event EventBeginPlay
  ;[0 1 0] BeginPlay
  (CallFunction|CalculateAccuracy)
  (CallFunction|Respawn)
  (Development|PrintString (Utilities|String|ToString(Integer) (Utilities|Array|Length (Variables|Default|GetGridBitMask))) true true "(R=0.000000,G=0.660000,B=1.000000,A=1.000000)" 22.0))

(event EventCurrentStateChange
  (params (CurrentProvider :type Object%20Object%20Reference) (ElectricalState :type Boolean) (CurrentFlow :type Float%20%28single-precision%29))
  ;[1 1 1] Set Max Targets
)

(fn ConstructionScript
  (bind _gridspacing (Variables|Default|GetGridSpacing))
  (|CallParentFunction)
  (Transformation|SetRelativeLocation (Variables|Default|GetScene) (Math|Vector|MakeVector (* (* (Math|Conversions|ToFloat(Integer) (- (Variables|Default|GetGridRows) 1)) -0.5) _gridspacing) 0.0 (* _gridspacing (* (Math|Conversions|ToFloat(Integer) (- (Variables|Default|GetGridCollums) 1)) -0.5))) false false))

(fn GetIsTargetDestroyed
  (params (Destroyed :type Boolean))
  (return false))

(fn GetOldestIndex
  (for (_array_element _array_index) 0
    (if (> (Actor|GetGameTimeSinceCreation _array_element) (LocalVariables|GetOldestTime))
      (LocalVariables|SetOldestTime (Actor|GetGameTimeSinceCreation _array_element))
      (LocalVariables|SetOldestTargetIndex _array_index)))
  (return (LocalVariables|GetOldestTargetIndex)))