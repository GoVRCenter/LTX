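; Health pickup Blueprint that restores a player pawn or AI bot to full health.
; It overrides no startup logic; all behavior lives in CustomEffect, which casts the actor to Vive_PawnCharacter, then AI_Master_Bot.
; A target below the near-full threshold has Health set straight to 100 and the function returns false.
; It returns true when nothing is applied, either because health is already full or the actor is another type.
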(event EventBeginPlay
  (|CallParentFunction) ; This node is disabled and will not be called.\nDrag off pins to build functionality.
)

(fn ConstructionScript
  (|CallParentFunction))

(fn CustomEffect
  (params (Actor :type Actor%20Object%20Reference))
  (bind _asvive_pawn_character (Utilities|Casting|CastToVive_PawnCharacter Actor)
    (:then
      (if (> (Variables|/Game/VRExpansion/Vive/Vive_PawnCharacter.Vive_PawnCharacter_C|GetHealth _asvive_pawn_character) 99.980003)
        _
        (else
          (Variables|/Game/VRExpansion/Vive/Vive_PawnCharacter.Vive_PawnCharacter_C|SetHealth _asvive_pawn_character 1e+02)
          (return false))))
    (:CastFailed
      (bind _asai_master_bot (Utilities|Casting|CastToAI_Master_Bot Actor)
        (:then
          (if (> (Variables|/Game/Blueprints/AI/AI_Master_Bot.AI_Master_Bot_C|GetHealth _asai_master_bot) 99.900002)
            _
            (else
              (Variables|/Game/Blueprints/AI/AI_Master_Bot.AI_Master_Bot_C|SetHealth _asai_master_bot 1e+02)
              (return false))))
        (:CastFailed
          _))))
  (return true))