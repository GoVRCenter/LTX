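; Weapon spawner that keeps a set number of laser, submachine, beam and rocket launcher guns plus shields available for one team.
; It spawns on BeginPlay, then rechecks on a looping timer whose interval is randomized once at start.
; Each type has its own array; invalid entries are removed and replacements appended.
; New weapons spawn at per-type position components, offset along world Y by index, with the owning team assigned.
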(event Custom|SpawnNewGuns
  (bind _laserlauncher (Variables|Default|GetLaserLauncher))
  (bind _shields (Variables|Default|GetShields))
  (bind _laser (Variables|Default|GetLaser))
  (bind _submachine (Variables|Default|GetSubMachine))
  (bind _laserbeam (Variables|Default|GetLaserBeam))
  (bind _pistolpos1 (Variables|Default|GetPistolPos1))
  (bind _numberofeachtokeepalive (Variables|Default|GetNumberOfEachToKeepAlive))
  (bind _submachinepos (Variables|Default|GetSubMachinePos))
  (bind _shieldpos (Variables|Default|GetShieldPos))
  (bind _beampos (Variables|Default|GetBeamPos))
  (bind _launcherpos (Variables|Default|GetLauncherPos))
  (bind _returnvalue (- _numberofeachtokeepalive 1))
  ;[1 1 1] Check Live Weapons
  (Utilities|FlowControl|Sequence
    (:then_0
      (for _index (range 0 _returnvalue)
        (Utilities|IsValid (Utilities|Array|Get(acopy) _laser _index)
          (:Is%20Not%20Valid
            (Utilities|Array|RemoveIndex _laser _index)
            (bind _returnvalue_2 (Game|SpawnActorfromClass "/Game/Blueprints/Weapons/BP_Weapon_Gun_Laser.BP_Weapon_Gun_Laser_C" (Math|Transform|MakeTransform (+ (Transformation|GetWorldLocation _pistolpos1) (Math|Vector|MakeVector 0.0 (* _index 2e+01) 0.0)) (Variables|/Script/Engine.SceneComponent|GetRelativeRotation _pistolpos1)) "Undefined" 0 (Variables|Default|GetTeamToSpawn) 0))
            (Utilities|Array|Add (Variables|Default|GetLaser) _returnvalue_2)))))
    (:then_1
      (for _index_2 (range 0 _returnvalue)
        (Utilities|IsValid (Utilities|Array|Get(acopy) _submachine _index_2)
          (:Is%20Not%20Valid
            (Utilities|Array|RemoveIndex _submachine _index_2)
            (bind _returnvalue_3 (Game|SpawnActorfromClass "/Game/Blueprints/Weapons/BP_Weapon_Gun_SubMachine.BP_Weapon_Gun_SubMachine_C" (Math|Transform|MakeTransform (+ (Transformation|GetWorldLocation _submachinepos) (Math|Vector|MakeVector 0.0 (* _index_2 2e+01) 0.0)) (Variables|/Script/Engine.SceneComponent|GetRelativeRotation _submachinepos)) "Undefined" 0 (Variables|Default|GetTeamToSpawn) 0))
            (Utilities|Array|Add (Variables|Default|GetSubMachine) _returnvalue_3)))))
    (:then_2
      (for _index_3 (range 0 _returnvalue)
        (Utilities|IsValid (Utilities|Array|Get(acopy) _laserbeam _index_3)
          (:Is%20Not%20Valid
            (Utilities|Array|RemoveIndex _laserbeam _index_3)
            (bind _returnvalue_4 (Game|SpawnActorfromClass "/Game/Blueprints/Weapons/BP_Weapon_Gun_LaserBeam.BP_Weapon_Gun_LaserBeam_C" (Math|Transform|MakeTransform (+ (Transformation|GetWorldLocation _beampos) (Math|Vector|MakeVector 0.0 (* _index_3 2e+01) 0.0)) (Variables|/Script/Engine.SceneComponent|GetRelativeRotation _beampos)) "Undefined" 0 (Variables|Default|GetTeamToSpawn) 0))
            (Utilities|Array|Add (Variables|Default|GetLaserBeam) _returnvalue_4)))))
    (:then_3
      (for _index_4 (range 0 _returnvalue)
        (Utilities|IsValid (Utilities|Array|Get(acopy) _laserlauncher _index_4)
          (:Is%20Not%20Valid
            (Utilities|Array|RemoveIndex _laserlauncher _index_4)
            (bind _returnvalue_5 (Game|SpawnActorfromClass "/Game/Blueprints/Weapons/BP_Weapon_Gun_Rocket_Launcher.BP_Weapon_Gun_Rocket_Launcher_C" (Math|Transform|MakeTransform (+ (Transformation|GetWorldLocation _launcherpos) (Math|Vector|MakeVector 0.0 (* _index_4 2e+01) 0.0)) (Variables|/Script/Engine.SceneComponent|GetRelativeRotation _launcherpos)) "Undefined" 0 (Variables|Default|GetTeamToSpawn) 0))
            (Utilities|Array|Add (Variables|Default|GetLaserLauncher) _returnvalue_5)))))
    (:then_4
      (for _index_5 (range 0 _returnvalue)
        (Utilities|IsValid (Utilities|Array|Get(acopy) _shields _index_5)
          (:Is%20Not%20Valid
            (Utilities|Array|RemoveIndex _shields _index_5)
            (bind _returnvalue_6 (Game|SpawnActorfromClass "/Game/Blueprints/Weapons/BP_Weapon_Shield.BP_Weapon_Shield_C" (Math|Transform|MakeTransform (+ (Transformation|GetWorldLocation _shieldpos) (Math|Vector|MakeVector 0.0 (* _index_5 2e+01) 0.0)) (Math|Rotator|CombineRotators "0,90.000000, 0" (Transformation|GetWorldRotation _shieldpos))) "Undefined" 0 (Variables|Default|GetTeamToSpawn) 0))
            (Utilities|Array|Add (Variables|Default|GetShields) _returnvalue_6)))))))

(event EventBeginPlay
  ;[0 1 0.1172] Begin Play
  (CallFunction|SpawnNewGuns)
  (Utilities|Time|SetTimerbyEvent (delegate Custom|SpawnNewGuns) (Math|Random|RandomFloatinRange 4.0 6.0) true))

(fn ConstructionScript)