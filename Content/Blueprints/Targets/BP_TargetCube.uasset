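; BP_TargetCube is a cube target that implodes and is destroyed when it takes any damage.
; Damage disables the cube's collision, then the Implosion timeline scales the actor from its captured X scale, applied uniformly.
; When the timeline finishes, the TargetDied dispatcher fires with the target's Index before the actor is destroyed.
; A randomized Lifetime auto-implosion is disconnected and never runs, and GetIsTargetDestroyed always returns false.
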(event EventBeginPlay)

(event Game|Damage|EventAnyDamage
  (params (Damage :type Float%20%28single-precision%29) (DamageType :type Damage%20Type%20Object%20Reference) (InstigatedBy :type Controller%20Object%20Reference) (DamageCauser :type Actor%20Object%20Reference))
  (Collision|SetCollisionEnabled (Variables|Default|GetCube) "NoCollision")
  (Variables|Default|SetActorScale (.x (Transformation|GetActorScale3D)))
  (bind _implosion (Timeline|Implosion Play)
    (:Update
      (Transformation|SetActorScale3D (Math|Vector|MakeVector (* _implosion (Variables|Default|GetActorScale)) (* _implosion (Variables|Default|GetActorScale)) (* _implosion (Variables|Default|GetActorScale)))))
    (:Finished
      (Default|CallTargetDied (Variables|Default|GetIndex))
      (Actor|DestroyActor))))

(fn ConstructionScript)

(fn GetIsTargetDestroyed
  (params (Destroyed :type Boolean))
  (return false))