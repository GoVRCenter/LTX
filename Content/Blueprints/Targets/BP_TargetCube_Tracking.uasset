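; BP_TargetCube_Tracking is a strafing cube target that counts hits, likely for tracking-aim practice.
; On BeginPlay it scales the cube by TargetScale and caches the world positions of two strafe points.
; The StrafePattern timeline then moves the actor between them by lerp, with alpha divided by SpeedDiviser.
; Any damage event increments HitScore and updates the Score text, regardless of damage amount.
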(event EventBeginPlay
  (bind _targetscale (Variables|Default|GetTargetScale))
  (Transformation|SetRelativeScale3D (Variables|Default|GetCube) (Math|Vector|MakeVector _targetscale _targetscale _targetscale))
  (Variables|Default|SetA (Transformation|GetWorldLocation (Variables|Default|GetStrafePoint1)))
  (Variables|Default|SetB (Transformation|GetWorldLocation (Variables|Default|GetStrafePoint2)))
  (bind _strafepattern (Timeline|StrafePattern Play)
    (:Update
      (Transformation|SetActorLocation (Math|Vector|Lerp(Vector) (Variables|Default|GetA) (Variables|Default|GetB) (/ _strafepattern (Variables|Default|GetSpeedDiviser))) false false))))

(event Game|Damage|EventAnyDamage
  (params (Damage :type Float%20%28single-precision%29) (DamageType :type Damage%20Type%20Object%20Reference) (InstigatedBy :type Controller%20Object%20Reference) (DamageCauser :type Actor%20Object%20Reference))
  (bind _result (Math|Float|IncrementFloat (Variables|Default|GetHitScore))
    (:%20%20
      (Rendering|Components|TextRender|SetText (Variables|Default|GetScore) (Utilities|Text|ToText(Float) _result "HalfToEven")))))

(fn ConstructionScript
  (|CallParentFunction))