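; BP_Weapon_Shield is a shield weapon that projects a force field while in use.
; OnUsed activates a radial force, plays click and pulsing audio, and runs a timeline that drives both the force field's uniform scale and the pulse volume.
; OnEndUsed deactivates the force, replays the click, stops the pulse audio and reverses the timeline to animate the field back.
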(event EventBeginPlay
  (|CallParentFunction) ; This node is disabled and will not be called.\nDrag off pins to build functionality.
)

(event EventOnUsed
  (Components|Activation|SetActive (Variables|Default|GetRadialForce) true true)
  (Audio|Components|Audio|Play (Variables|Default|GetAudio_Pulsate) 0.0)
  (bind _animation (Timeline|Timeline_0_0 Play)
    (:Update
      (Transformation|SetRelativeScale3D (Variables|Default|GetForceField) (Math|Vector|MakeVector _animation _animation _animation))
      (Audio|Components|Audio|SetVolumeMultiplier (Variables|Default|GetAudio_Pulsate) _animation :!class /Script/Engine.AudioComponent))))

(event EventOnEndUsed
  (Components|Activation|SetActive (Variables|Default|GetRadialForce) false false)
  (Audio|Components|Audio|Play (Variables|Default|GetAudio_Click) 0.0)
  (Audio|Components|Audio|Stop (Variables|Default|GetAudio_Pulsate))
  (bind _animation (Timeline|Timeline_0_0 Reverse)
    (:Update
      (Transformation|SetRelativeScale3D (Variables|Default|GetForceField) (Math|Vector|MakeVector _animation _animation _animation))
      (Audio|Components|Audio|SetVolumeMultiplier (Variables|Default|GetAudio_Pulsate) _animation :!class /Script/Engine.AudioComponent))))

(fn ConstructionScript
  (|CallParentFunction))