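; Lab elevator lift Blueprint that raises and lowers a flat wall panel mesh in response to electrical current.
; CurrentStateChange calls Up when the electrical state is on with positive current flow, and Down otherwise.
; Up plays the ElevatorAnimation timeline, whose Movement track scaled by TravelDistance sets the panel's relative Z location.
; Down reverses the same timeline.
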(event Custom|Up
  ;[1 1 1] Up and Down Events
  ;[1 1 1] Animation Timeline
  (bind _movement (Timeline|ElevatorAnimation Play)
    (:Update
      ;[1 1 1] Set Elevator Relative Location
      (Transformation|SetRelativeLocation (Variables|Default|GetSM_Wall_Panel_Flat) (Math|Vector|MakeVector 0.0 0.0 (* _movement (Variables|Default|GetTravelDistance))) false false))))

(event Custom|Down
  ;[1 1 1] Up and Down Events
  ;[1 1 1] Animation Timeline
  (bind _movement (Timeline|ElevatorAnimation Reverse)
    (:Update
      ;[1 1 1] Set Elevator Relative Location
      (Transformation|SetRelativeLocation (Variables|Default|GetSM_Wall_Panel_Flat) (Math|Vector|MakeVector 0.0 0.0 (* _movement (Variables|Default|GetTravelDistance))) false false))))

(event EventCurrentStateChange
  (params (CurrentProvider :type Object%20Object%20Reference) (ElectricalState :type Boolean) (CurrentFlow :type Float%20%28single-precision%29))
  ;[1 1 1] Event Current
  (if (and ElectricalState (> CurrentFlow 0.0))
    (CallFunction|Up)
    (else
      (CallFunction|Down))))

(fn ConstructionScript)