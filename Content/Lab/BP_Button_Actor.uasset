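; BP_Button_Actor is a button that passes its on/off state to linked electrical targets.
; The construction script copies the actor's ButtonType onto its ButtonComp component.
; CurrentStateChange stores the current flow reaching the button without forwarding it.
; When ButtonComp changes state, the actor sends every entry in ElectricalTargets a CurrentStateChangeMessage interface call carrying itself as provider, the button state and the stored flow.
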(event OnButtonStateChanged(ButtonComp)
  (params (ButtonState :type Boolean) (InteractingActor :type Actor%20Object%20Reference) (InteractingComponent :type Primitive%20Component%20Object%20Reference))
  ;[1 1 1] Send Out Electrical Interface Call
  (for _array_element (Variables|Default|GetElectricalTargets)
    (Class|ElectricalObject|CurrentStateChange(Message) _array_element self ButtonState (Variables|Default|GetCurrentFlow))))

(event EventCurrentStateChange
  (params (CurrentProvider :type Object%20Object%20Reference) (ElectricalState :type Boolean) (CurrentFlow :type Float%20%28single-precision%29))
  ;[1 1 1] Electrical Current Event
  (Variables|Default|SetCurrentFlow CurrentFlow))

(fn ConstructionScript
  (Variables|/Script/VRExpansionPlugin.VRButtonComponent|SetButtonType (Variables|Default|GetButtonComp) (Variables|Default|GetButton%20Type)))