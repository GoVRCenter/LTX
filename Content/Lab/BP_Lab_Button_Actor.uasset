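; BP_Lab_Button_Actor is a lab button that acts as a node in an electrical circuit, passing its state on to connected targets.
; The construction script copies the actor's ButtonType to its ButtonComp component.
; When the component reports a state change, it messages every ElectricalTarget with that state and the stored CurrentFlow.
; Incoming electrical state changes only update its stored CurrentFlow and ButtonState, without forwarding them.
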(event OnButtonStateChanged(ButtonComp)
  (params (ButtonState :type Boolean) (InteractingActor :type Actor%20Object%20Reference) (InteractingComponent :type Primitive%20Component%20Object%20Reference))
  ;[1 1 1] Electrical Interface Events
  (for _array_element (Variables|Default|GetElectricalTargets)
    (Class|ElectricalObject|CurrentStateChange(Message) _array_element self ButtonState (stale EventCurrentStateChange _output_get))))

(event EventCurrentStateChange
  (params (CurrentProvider :type Object%20Object%20Reference) (ElectricalState :type Boolean) (CurrentFlow :type Float%20%28single-precision%29))
  ;[1 1 1] Electrical Interface Events
  (bind _output_get (Variables|Default|SetCurrentFlow CurrentFlow))
  (Variables|Default|SetButtonState ElectricalState))

(fn ConstructionScript
  (Variables|/Script/VRExpansionPlugin.VRButtonComponent|SetButtonType (Variables|Default|GetButtonComp) (Variables|Default|GetButton%20Type)))