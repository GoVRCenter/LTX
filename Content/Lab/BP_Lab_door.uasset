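; Lab door Blueprint that slides vertically in response to electrical state changes and is colored for the Red or Blue team.
; CurrentStateChange plays the door audio and runs a timeline forward when powered or in reverse when not, driving the door's relative Z, with CurrentFlow setting the play rate.
; The construction script picks the team's tile material.
; OnRep_IsOpen is empty, with unconnected server open/close logic.
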(event EventCurrentStateChange
  (params (CurrentProvider :type Object%20Object%20Reference) (ElectricalState :type Boolean) (CurrentFlow :type Float%20%28single-precision%29))
  (bind _audio (Variables|Default|GetAudio))
  (Components|Timeline|SetPlayRate (Variables|Default|GetTimeline_Animation) CurrentFlow)
  (if ElectricalState
    ;[1 1 1] Play Audio
    (Audio|Components|Audio|Play _audio 0.0)
    ;[1 1 1] Animation
    (bind _movement (Timeline|Timeline_Animation Play)
      (:Update
        ;[1 1 1] Set Relative Z Location
        (Transformation|SetRelativeLocation (Variables|Default|GetDoor) (Math|Vector|MakeVector 0.0 0.0 _movement) false false)))
    (else
      (Audio|Components|Audio|Play _audio 0.0)
      (Timeline|Timeline_Animation Reverse))))

(fn ConstructionScript
  (bind _door (Variables|Default|GetDoor))
  (switch Utilities|FlowControl|Switch|SwitchonEnum_Teams (Variables|Default|GetTeam)
    (:NewEnumerator0
      (Rendering|Material|SetMaterial _door 0 "/Game/Materials/MI_Concrete_Light_Tiles_Red.MI_Concrete_Light_Tiles_Red"))
    (:NewEnumerator1
      (Rendering|Material|SetMaterial _door 0 "/Game/Materials/MI_Concrete_Light_Tiles_Blue.MI_Concrete_Light_Tiles_Blue"))))

(fn OnRepIsOpen)