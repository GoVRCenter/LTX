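; BP_DamagableCube is a damage test actor: a cube that loses health and gets pushed when hit by point damage.
; PointDamage subtracts from Health, updates the HealthIndicator text, applies a fixed-strength impulse at the hit location against the hit normal, and prints the impact normal for debugging.
; The construction script shows the starting Health on the indicator.
; Health has no lower limit or death handling.
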(event Game|Damage|EventPointDamage
  (params (Damage :type Float%20%28single-precision%29) (DamageType :type Damage%20Type%20Object%20Reference) (HitLocation :type Vector :default "0, 0, 0") (HitNormal :type Vector :default "0, 0, 0") (HitComponent :type Primitive%20Component%20Object%20Reference) (BoneName :type Name :default "None") (ShotFromDirection :type Vector :default "0, 0, 0") (InstigatedBy :type Controller%20Object%20Reference) (DamageCauser :type Actor%20Object%20Reference) (HitInfo :type Hit%20Result%20Structure%20%28by%20ref%29))
  (Utilities|FlowControl|Sequence
    (:then_0
      (bind _output_get (Variables|Default|SetHealth (- (Variables|Default|GetHealth) Damage)))
      (Rendering|Components|TextRender|SetText (Variables|Default|GetHealthIndicator) (Utilities|Text|ToText(Float) _output_get "HalfToEven")))
    (:then_1
      (Physics|AddImpulseatLocation (Variables|Default|GetCube) (* (Math|Vector|NegateVector HitNormal) 5e+03) HitLocation "None"))
    (:then_2
      (Development|PrintString (Utilities|String|ToString(Vector) (.impactnormal HitInfo)) true true "(R=0.000000,G=0.660000,B=1.000000,A=1.000000)" 1e+01))))

(fn ConstructionScript
  (Rendering|Components|TextRender|SetText (Variables|Default|GetHealthIndicator) (Utilities|Text|ToText(Float) (Variables|Default|GetHealth) "HalfToEven")))