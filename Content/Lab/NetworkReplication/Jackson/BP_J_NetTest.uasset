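; BP_J_NetTest is a grippable test actor in the network replication lab, with no gameplay logic of its own.
; It implements VR grip interface functions that return fixed values, and its construction script is empty.
; It allows a single interactive physics-collision grip with late updates always on, keeps original movement replication, and teleports all components.
; It offers no secondary grip, slots, socketing or drop simulation, and always reports itself as not held.
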(fn ConstructionScript)

(fn TeleportBehavior
  (return "TeleportAllComponents"))

(fn SimulateonDrop
  (return false))

(fn SecondaryGripType
  (return "SG_None"))

(fn RequestsSocketing
  (return 0 "None" "" false))

(fn IsHeld
  (return 0 false))

(fn GripMovementReplicationType
  (return "KeepOriginalMovement"))

(fn GripLateUpdateSetting
  (return "LateUpdatesAlwaysOn"))

(fn GripBreakDistance
  (return 0.0))

(fn GetPrimaryGripType
  (params (bIsSlot :type Boolean))
  (return "InteractiveCollisionWithPhysics"))

(fn GetGripStiffnessandDamping
  (return 0.0 0.0))

(fn GetGripScripts
  (return 0 false))

(fn DenyGripping
  (params (GripInitiator :type Grip%20Motion%20Controller%20Component%20Object%20Reference))
  (return false))

(fn ClosestGripSlotinRange
  (params (WorldLocation :type Vector :default "0, 0, 0") (bSecondarySlot :type Boolean) (CallingController :type Grip%20Motion%20Controller%20Component%20Object%20Reference) (OverridePrefix :type Name :default "None"))
  (return false "" "None"))

(fn AllowsMultipleGrips
  (return false))

(fn AdvancedGripSettings
  (return ""))