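; A blank canvas actor that owns a runtime render target which brush materials can paint onto.
; On BeginPlay it creates a 1024-square render target and a dynamic instance of the static mesh's material, then feeds the target into that instance as a texture parameter.
; The DrawBrushtoRenderTarget interface event draws the supplied brush material into the render target shown through the mesh's material.
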(event EventBeginPlay
  (bind _staticmesh (Variables|Default|GetStaticMesh))
  ;[0 1 0] Begin Play
  (bind _returnvalue (Rendering|CreateRenderTarget2D 1024 1024 "RTF_RGBA8"))
  (Variables|Default|SetyourMom _returnvalue)
  (bind _returnvalue_2 (Rendering|Material|CreateDynamicMaterialInstance (Rendering|Material|GetMaterial _staticmesh 0) "None" "None" :!class /Script/Engine.KismetMaterialLibrary))
  (bind _output_get (Variables|Default|SetyourDad _returnvalue_2))
  (Rendering|Material|SetMaterial _staticmesh 0 _output_get)
  (Rendering|Material|SetTextureParameterValue _output_get "yourSister" (Variables|Default|GetyourMom)))

(event EventDrawBrushtoRenderTarget
  (params (BrushMaterial :type Material%20Instance%20Dynamic%20Object%20Reference%20%28by%20ref%29))
  ;[1 1 1] Interface Events
  (Rendering|DrawMaterialtoRenderTarget (Variables|Default|GetyourMom) BrushMaterial))

(fn ConstructionScript)