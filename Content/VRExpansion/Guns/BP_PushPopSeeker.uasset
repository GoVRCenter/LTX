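; Grippable VR push-pop that launches along the holder's camera forward vector with a strong spin when released.
; Grip caches whether the holder is locally controlled, so that client applies force and torque itself on release.
; The authority also applies them unless it is a dedicated server, and sends them through Multi_ApplyForces, which skips the locally controlled holder.
; Seeking is unimplemented: Tick loops over TargetDetectionSphere overlaps without acting.
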(event Custom|Multi_ApplyForces
  (params (Force :type Vector%20Net%20Quantize%20Structure) (Torque :type Vector%20Net%20Quantize%20Structure))
  (bind _staticmeshcomponent (Variables|Default|GetStaticMeshComponent))
  (if (not (Variables|Default|GetLocallyControlled))
    (Physics|AddForce _staticmeshcomponent Force "None" false)
    (Class|PrimitiveComponent|AddTorqueinDegrees _staticmeshcomponent Torque "None" false)))

(event EventBeginPlay
  (|CallParentFunction) ; This node is disabled and will not be called.\nDrag off pins to build functionality.
)

(event Collision|EventActorBeginOverlap
  (params (OtherActor :type Actor%20Object%20Reference))
  (|CallParentFunction OtherActor) ; This node is disabled and will not be called.\nDrag off pins to build functionality.
)

(event EventTick
  (params (DeltaSeconds :type Float%20%28single-precision%29))
  (|CallParentFunction DeltaSeconds)
  (Utilities|Array|ForEachLoopwithBreak (Collision|GetOverlappingActors (Variables|Default|GetTargetDetectionSphere) "/Game/VRExpansion/Guns/Dummy.Dummy_C" :!class /Script/Engine.PrimitiveComponent)))

(event EventOnGripRelease
  (params (ReleasingController :type Grip%20Motion%20Controller%20Component%20Object%20Reference) (GripInformation :type BP%20Actor%20Grip%20Information%20Structure%20%28by%20ref%29) (bWasSocketed :type Boolean))
  (bind _returnvalue (Components|GetOwner ReleasingController))
  (bind _staticmeshcomponent (Variables|Default|GetStaticMeshComponent))
  (bind _staticmeshcomponent_2 (Variables|Default|GetStaticMeshComponent))
  (bind _staticmeshcomponent_3 (Variables|Default|GetStaticMeshComponent))
  (bind _returnvalue_2 (Math|Vector|GetRightVector _staticmeshcomponent_2))
  (bind _returnvalue_3 (* _returnvalue_2 8e+07))
  (Networking|SwitchHasAuthority
    (:Authority
      (bind _asvrcharacter (Utilities|Casting|CastToVRCharacter _returnvalue))
      (CallFunction|MultiApplyForces (Class|VRExpansionFunctionLibrary|ToFVectorNetQuantize(FVector) (* (Math|Vector|GetForwardVector (Variables|/Script/VRExpansionPlugin.VRBaseCharacter|GetVRReplicatedCamera _asvrcharacter)) 1e+05)) (Class|VRExpansionFunctionLibrary|ToFVectorNetQuantize(FVector) _returnvalue_3))
      (if (not (Networking|IsDedicatedServer))
        (Physics|AddForce _staticmeshcomponent_3 (* (Math|Vector|GetForwardVector (Variables|/Script/VRExpansionPlugin.VRBaseCharacter|GetVRReplicatedCamera _asvrcharacter)) 1e+05) "None" false)
        (Class|PrimitiveComponent|AddTorqueinDegrees _staticmeshcomponent_3 _returnvalue_3 "None" false)))
    (:Remote
      (bind _asvrcharacter_2 (Utilities|Casting|CastToVRCharacter _returnvalue))
      (if (Variables|Default|GetLocallyControlled)
        (Physics|AddForce _staticmeshcomponent (* (Math|Vector|GetForwardVector (Variables|/Script/VRExpansionPlugin.VRBaseCharacter|GetVRReplicatedCamera _asvrcharacter_2)) 1e+05) "None" false)
        (Class|PrimitiveComponent|AddTorqueinDegrees _staticmeshcomponent (* (Math|Vector|GetRightVector (Variables|Default|GetStaticMeshComponent)) 8e+07) "None" false)))))

(event EventOnGrip
  (params (GrippingController :type Grip%20Motion%20Controller%20Component%20Object%20Reference) (GripInformation :type BP%20Actor%20Grip%20Information%20Structure%20%28by%20ref%29))
  (bind _aspawn (Utilities|Casting|CastToPawn (Components|GetOwner GrippingController)))
  (Variables|Default|SetLocallyControlled (Pawn|IsLocallyControlled _aspawn)))

(fn ConstructionScript
  (|CallParentFunction))

(fn MultiApplyForces
  (params (Force1 :type Vector%20Net%20Quantize%20Structure) (Torque1 :type Vector%20Net%20Quantize%20Structure)))