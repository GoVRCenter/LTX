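; BP_Lever_ActorLever is a test lever actor for VR, built around a VRLever component.
; Its only active logic prints the lever angle whenever the component reports a state change.
; GetAngle reads the lever's roll, both raw and relative to InitialRot.
; Leftover grip, angle-update, drive and drop-at-target logic is disconnected and never runs.
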(event OnLeverStateChanged(VRLever)
  (params (LeverStatus :type Boolean) (LeverStatusType :type EVRInteractibleLeverEventType%20Enum :default "LeverPositive") (LeverAngleAtTime :type Float%20%28single-precision%29) (FullLeverAngleAtTime :type Float%20%28single-precision%29))
  (Development|PrintString (Utilities|String|ToString(Float) LeverAngleAtTime)))

(event EventBeginPlay
  ;[0.005598 0.224 0.03015] Begin Play
)

(event EventTick
  (params (DeltaSeconds :type Float%20%28single-precision%29))
  ;[0.2656 0 0] Tick
)

(event EventCurrentStateChange
  (params (CurrentProvider :type Object%20Object%20Reference) (ElectricalState :type Boolean) (CurrentFlow :type Float%20%28single-precision%29)))

(fn ConstructionScript)

(fn GetAngle
  (bind _vrlever (Variables|Default|GetVRLever))
  (bind _relativerotation (Variables|/Script/Engine.SceneComponent|GetRelativeRotation _vrlever))
  (return (- (.roll _relativerotation) (Variables|Default|GetInitialRot)) (.roll _relativerotation)))